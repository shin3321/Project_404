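; BP_MainGate is a gate actor that swings open or closed when toggled through a GateInterface event.
; A box overlap sets CanOpenDoor, so toggling works only while that flag is set and the gate is not moving.
; The toggle flips IsOpen, whose RepNotify plays or reverses the OpenDoor timeline.
; The timeline lerps the mesh's relative rotation and holds IsOpening until it finishes.
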(event `/Game/Project404/Game/BPI_Interactable.GateInterface`
  (if (`self.bIsOpening`)
    _
    (elif (`self.bCanOpenDoor`)
      (if (`self.bIsOpen`)
        (set `self.bIsOpen` false)
        (else
          (set `self.bIsOpen` true))))))

(event `self.Box.OnComponentBeginOverlap`
  (params (OverlappedComponent :type "PrimitiveComponent Object Reference") (OtherActor :type "Actor Object Reference") (OtherComp :type "PrimitiveComponent Object Reference") (OtherBodyIndex :type Integer) (bFromSweep :type Boolean) (SweepResult :type "HitResult Structure (by ref)"))
  (set `self.bCanOpenDoor` true))

(event `self.Box.OnComponentEndOverlap`
  (params (OverlappedComponent :type "PrimitiveComponent Object Reference") (OtherActor :type "Actor Object Reference") (OtherComp :type "PrimitiveComponent Object Reference") (OtherBodyIndex :type Integer))
  (set `self.bCanOpenDoor` false))

(fn `OnRep_bIsOpen`
  (if (`self.bIsOpen`)
    (`TimelineComponent.Play` (`self.OpenDoor`))
    (else
      (`TimelineComponent.Reverse` (`self.OpenDoor`)))))

(fn `UserConstructionScript`)
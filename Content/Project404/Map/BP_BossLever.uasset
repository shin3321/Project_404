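; BP_BossLever is a one-shot lever that flags entry into the boss level.
; Box overlap toggles whether it can be pulled, and the GateInterface event then latches IsEnterBoss and sets EnterBossLevel on the FZFGameInstance.
; The IsEnterBoss RepNotify plays the DownLever timeline, whose update lerps the lever mesh's rotation.
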(event `/Game/Project404/Game/BPI_Interactable.GateInterface`
  (if (`self.bIsEnterBoss`)
    _
    (elif (`self.bCanLever`)
      (set `self.bIsEnterBoss` true)
      (bind _asfzfgame_instance (cast `FZFGameInstance` (`GameplayStatics.GetGameInstance`)))
      (`/Engine/EditorBlueprintResources/StandardMacros.IsValid` _asfzfgame_instance
        (:`Is Valid`
          (set `FZFGameInstance.bEnterBossLevel` true _asfzfgame_instance))))))

(event `self.Box.OnComponentBeginOverlap`
  (params (OverlappedComponent :type "PrimitiveComponent Object Reference") (OtherActor :type "Actor Object Reference") (OtherComp :type "PrimitiveComponent Object Reference") (OtherBodyIndex :type Integer) (bFromSweep :type Boolean) (SweepResult :type "HitResult Structure (by ref)"))
  (set `self.bCanLever` true))

(event `self.Box.OnComponentEndOverlap`
  (params (OverlappedComponent :type "PrimitiveComponent Object Reference") (OtherActor :type "Actor Object Reference") (OtherComp :type "PrimitiveComponent Object Reference") (OtherBodyIndex :type Integer))
  (set `self.bCanLever` false))

(fn `OnRep_bIsEnterBoss`
  (`TimelineComponent.Play` (`self.DownLever`)))

(fn `UserConstructionScript`)
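; BP_DoubleDoor is a door with upper and lower panels that slide apart and back together vertically.
; An overlap box sets whether it can be operated, and the GateInterface event then toggles IsDoorOpen.
; The OnRep for that state plays or reverses the OpenDoor timeline, which lerps both panels' relative locations.
; A separate CloseDoor timeline exists but is never played.
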(event `/Game/Project404/Game/BPI_Interactable.GateInterface`
  (if (`self.bCanOpenDoor`)
    (if (`self.bIsDoorOpen`)
      (set `self.bIsDoorOpen` false)
      (else
        (set `self.bIsDoorOpen` true)))))

(event `self.Box.OnComponentBeginOverlap`
  (params (OverlappedComponent :type "PrimitiveComponent Object Reference") (OtherActor :type "Actor Object Reference") (OtherComp :type "PrimitiveComponent Object Reference") (OtherBodyIndex :type Integer) (bFromSweep :type Boolean) (SweepResult :type "HitResult Structure (by ref)"))
  (set `self.bCanOpenDoor` true))

(event `self.Box.OnComponentEndOverlap`
  (params (OverlappedComponent :type "PrimitiveComponent Object Reference") (OtherActor :type "Actor Object Reference") (OtherComp :type "PrimitiveComponent Object Reference") (OtherBodyIndex :type Integer))
  (set `self.bCanOpenDoor` false))

(fn `OnRep_bIsDoorOpen`
  (if (`self.bIsDoorOpen`)
    (`TimelineComponent.Play` (`self.OpenDoor`))
    (else
      (`TimelineComponent.Reverse` (`self.OpenDoor`)))))

(fn `UserConstructionScript`
  (`parent.UserConstructionScript`))